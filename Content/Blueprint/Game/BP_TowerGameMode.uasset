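; Tower game mode that spawns enemies and keeps the enemy counts in TowerGameState up to date.
; SpawnEnemy creates a BP_EnemyBase at the first TargetPoint tagged "Start", decrements the pending spawn count and calls StopSpawningEnemy once it reaches zero.
; Each spawned enemy's OnDeath is bound to a handler that decrements the remaining enemy count.
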(event `self.SpawnEnemy`
  (bind _outactors (`GameplayStatics.GetAllActorsOfClassWithTag` "/Script/Engine.TargetPoint" "Start"))
  (bind _returnvalue (`|SpawnActorFromClass` "/Game/Blueprint/Actor/Enemy/BP_EnemyBase.BP_EnemyBase_C" (`self.GetTransform` (`|GetArrayItem` _outactors)) "Undefined" "MultiplyWithRoot" null null))
  (bind _result (`/Engine/EditorBlueprintResources/StandardMacros.DecrementInt` (`TowerGameState.EnemiesPendingSpawn` (`self.TowerGameState`)))
    (:`  `
      (if (<= _result 0)
        (`self.StopSpawningEnemy`))
      (add `TowerEnemyPawn.OnDeath` _returnvalue (delegate `OnDeath_Event`)))))

(event `OnDeath_Event`
  (params (EnemyPawn :type "TowerEnemyPawn Object Reference"))
  (`/Engine/EditorBlueprintResources/StandardMacros.DecrementInt` (`TowerGameState.RemainingEnemyCount` (`self.TowerGameState`))))

(fn `UserConstructionScript`)